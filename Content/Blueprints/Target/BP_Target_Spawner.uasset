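; Spawner actor that populates a box area with BP_target actors, keeping their count in the level capped.
; StartSpawning, which is not called from BeginPlay, spawns an initial burst and starts a looping timer for SpawnTarget.
; Each spawn picks a random point in SpawnArea, sized by the construction script, and rotates the target toward the player camera with a yaw offset.
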(event `self.ReceiveBeginPlay`)

(event `StartSpawning`
  ;[1 1 1] Start Spawing
  (`KismetSystemLibrary.K2_SetTimerDelegate` (delegate `SpawnTarget`) 1.0 true)
  (for _ (range 4)
    (`self.SpawnTarget`)))

(event `SpawnTarget`
  (bind _spawn_area (`self.Spawn_Area`))
  ;[1 1 1] Spawning Targets
  (bind _outactors (`GameplayStatics.GetAllActorsOfClass` "/Game/Blueprints/Target/BP_target.BP_target_C"))
  (if (< (`KismetArrayLibrary.Array_Length` _outactors) 10)
    (bind _output_get (set `self.SpawnLocation` (`KismetMathLibrary.RandomPointInBoundingBox` (`SceneComponent.K2_GetComponentLocation` _spawn_area) (`BoxComponent.GetScaledBoxExtent` _spawn_area))))
    (bind (_returnvalue_roll _returnvalue_pitch _returnvalue_yaw) (`KismetMathLibrary.BreakRotator` (`KismetMathLibrary.FindLookAtRotation` _output_get (`SceneComponent.K2_GetComponentLocation` (`PlayerCameraManager.TransformComponent` (`GameplayStatics.GetPlayerCameraManager` 0))))))
    (`|SpawnActorFromClass` "/Game/Blueprints/Target/BP_target.BP_target_C" (`KismetMathLibrary.MakeTransform` _output_get (`KismetMathLibrary.MakeRotator` _returnvalue_roll _returnvalue_pitch (- _returnvalue_yaw 90.0))) "AdjustIfPossibleButAlwaysSpawn" "OverrideRootScale" null null)))

(fn `UserConstructionScript`
  (`BoxComponent.SetBoxExtent` (`self.Spawn_Area`) (`self.In Box Extent`) true))